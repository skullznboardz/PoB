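; Player controller that relays jump, dash and horizontal walking input through event dispatcher calls.
; Every tick it also converts the Horizontal and Vertical axes into HDirection and VDirection values of -1, 0 or 1.
; A direction changes only past a high threshold or at exactly zero, so partial stick input keeps the previous value.
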(event `InputAction|Jump`
  (params (Key :type "Key Structure"))
  (:`Pressed`
    (`self.jumpPressed`))
  (:`Released`
    (`self.jumpReleased`)))

(event `InputAxis|Horizontal`
  (params (AxisValue :type "Float (single-precision)"))
  (`self.walkingInput` AxisValue))

(event `InputAction|Dash`
  (params (Key :type "Key Structure"))
  (:`Pressed`
    (`self.DashPressed`)))

(event `self.ReceiveTick`
  (params (DeltaSeconds :type "Float (single-precision)"))
  (`|ExecutionSequence`
    (:`then_0`
      (`self.Horizontal Check`))
    (:`then_1`
      (`self.Vertical Check`))))

(fn `Horizontal Check`
  (bind _returnvalue (`self.GetInputAxisValue`))
  (if (> _returnvalue 0.75)
    (set `self.H Direction` 1.0)
    (elif (< _returnvalue -0.75)
      (set `self.H Direction` -1.0)
      (elif (== _returnvalue 0.0)
        (set `self.H Direction` 0.0)))))

(fn `UserConstructionScript`)

(fn `Vertical Check`
  (bind _returnvalue (`self.GetInputAxisValue`))
  (if (> _returnvalue 0.75)
    (set `self.V Direction` 1.0)
    (elif (< _returnvalue -0.75)
      (set `self.V Direction` -1.0)
      (elif (== _returnvalue 0.0)
        (set `self.V Direction` 0.0)))))
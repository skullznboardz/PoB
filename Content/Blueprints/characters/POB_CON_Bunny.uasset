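; Player bunny character for a 2D side-scroller, with walk, run, jump, crouch, dash and damage handling; death only prints a message.
; Tick swaps flipbooks by movement state and snaps Y to zero during jumps.
; Hits on tagged walls or ceilings zero gravity and velocity until a jump launches away.
; Double jump and ground pound are flag-gated, noted as always false; dash fires from its button, as double-tap outputs are unconnected.
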(event `Lock Y Axis`
  (bind _y (.y (`self.K2_GetActorLocation`)))
  ;[1 1 1] Lock Y Axis
  (if (`self.hasJumped`)
    (if (or (< _y 0.0) (> _y 0.0))
      (`self.K2_SetActorTransform` (`KismetMathLibrary.MakeTransform` (`KismetMathLibrary.MakeVector` (.x (.location (`self.GetTransform`))) 0.0 (.z (.location (`self.GetTransform`)))) (.rotation (`self.GetTransform`)) (.scale (`self.GetTransform`))) true))))

(event `self.ReceiveBeginPlay`
  ;[1 1 1] Setup
  (set `self.CurrentLife` (`self.MaxLife`)))

(event `InputAction|Run`
  (params (Key :type "Key Structure"))
  ;[1 1 1] Horizontal Movement
  ;;[1 1 1] Running
  (:`Pressed`
    (set `self.isRunning` true)
    (set `self.RunningPlayRate` 2.0)
    (`PaperFlipbookComponent.SetPlayRate` (`self.b_idle`) (`self.RunningPlayRate`) :!label _label))
  (:`Released`
    (set `self.isRunning` false)
    (set `self.RunningPlayRate` 1.0)
    (goto _label)))

(event `InputAction|Jump`
  (params (Key :type "Key Structure"))
  (bind _jumpcount (`self.JumpCount`))
  ;[1 1 1] Jumping
  (:`Pressed`
    (set `self.hasJumped` true)
    (if (`self.isStuckToWall`)
      ;;[1 1 1] Wall Jump
      (set `self.isStuckToWall` false)
      (set `CharacterMovementComponent.GravityScale` 1.5 (`self.CharacterMovement`))
      (`self.LaunchCharacter` (`KismetMathLibrary.MakeVector` (* (`self.wall normal`) 1000.0) 0.0 1250.0))
      (elif (`self.Is Stuck on Ceiling`)
        ;;[1 1 1] Ceiling Jump
        (set `self.Is Stuck on Ceiling` false)
        (set `CharacterMovementComponent.GravityScale` 1.5 (`self.CharacterMovement`))
        (`self.LaunchCharacter` (`KismetMathLibrary.MakeVector` 0.0 0.0 (* (`self.ceiling normal`) 1000.0)))
        (else
          (set `self.JumpCount` (+ _jumpcount 1))
          (if (== _jumpcount 2)
            (if (`self.canDoubleJump`)
              (`self.LaunchCharacter` (0.0 0.0 750.0))
              (`PaperFlipbookComponent.SetFlipbook` (`self.b_idle`) "/Game/flipbook/character/bunny/b_jump.b_jump" :!label _label_2))
            (else
              (`self.Jump`)
              (goto _label_2))))))))

(event `InputAxis|Horizontal`
  (params (AxisValue :type "Float (single-precision)"))
  (bind _threshold (`self.Threshold`))
  ;[1 1 1] Horizontal Movement
  (if (`self.isStuckToWall`)
    _
    (elif (not (`self.Is Stuck on Ceiling`))
      (`self.SplitAxis` AxisValue _threshold
        (:`Positive`
          (set `self.isWalking` true :!label _label_3)
          (`SceneComponent.SetRelativeScale3D` (`self.b_idle`) (`KismetMathLibrary.MakeVector` AxisValue 1.0 1.0)))
        (:`Negative`
          (goto _label_3))
        (:`Neutral`
          (set `self.isWalking` false)))
      (`|ExecutionSequence`
        (:`then_0`
          (if (`self.isRunning`)
            (`self.AddMovementInput` (1.0 0.0 0.0) AxisValue)
            (else
              (`self.AddMovementInput` (0.5 0.0 0.0) AxisValue))))
        (:`then_1`
          (`self.AxisDoubleTap` AxisValue _threshold 0.4
            (:`Positive`
              _)
            (:`Negative`
              _))
          (`self.LaunchCharacter` (`KismetMathLibrary.MakeVector` (* AxisValue 1000.0) 0.0 250.0) :!label _label_4))))))

(event `InputAction|Dash`
  (params (Key :type "Key Structure"))
  ;[1 1 1] Horizontal Movement
  (:`Pressed`
    (goto _label_4)))

(event `self.ReceiveTick`
  (params (DeltaSeconds :type "Float (single-precision)"))
  (bind _b_idle (`self.b_idle`))
  ;[1 1 1] Jumping
  (`self.Lock Y Axis`)
  (if (`NavMovementComponent.IsFalling` (`self.CharacterMovement`))
    (if (`self.hasJumped`)
      (goto _label_2)
      (else
        (`PaperFlipbookComponent.SetFlipbook` _b_idle "/Game/flipbook/character/bunny/b_fall.b_fall")))
    (else
      (set `self.JumpCount` 0)
      (set `self.hasJumped` false)
      (set `self.isGroundPounding` false)
      (if (`self.isWalking`)
        (`PaperFlipbookComponent.SetFlipbook` _b_idle "/Game/flipbook/character/bunny/b_walk.b_walk")
        (else
          (`PaperFlipbookComponent.SetFlipbook` _b_idle "/Game/flipbook/character/bunny/b_idle.b_idle"))))))

(event `self.ReceiveAnyDamage`
  (params (Damage :type "Float (single-precision)") (DamageType :type "DamageType Object Reference") (InstigatedBy :type "Controller Object Reference") (DamageCauser :type "Actor Object Reference"))
  ;[1 1 1] Life, Death & Damage
  (bind _output_get (set `self.CurrentLife` (- (`self.CurrentLife`) Damage)))
  (if (<= _output_get 0.0)
    (`self.Death`)
    (else
      (`KismetSystemLibrary.PrintString` (`KismetStringLibrary.Concat_StrStr` "Remaining Life = " (`KismetStringLibrary.Conv_DoubleToString` _output_get))))))

(event `self.ReceiveHit`
  (params (MyComp :type "PrimitiveComponent Object Reference") (Other :type "Actor Object Reference") (OtherComp :type "PrimitiveComponent Object Reference") (bSelfMoved :type Boolean) (HitLocation :type "Vector Structure") (HitNormal :type "Vector Structure") (NormalImpulse :type "Vector Structure") (Hit :type "HitResult Structure (by ref)"))
  (bind _charactermovement (`self.CharacterMovement`))
  ;[1 1 1] Wall/Ceiling Jump Collisions Detection
  (if (`self.ActorHasTag` Other "Wall")
    (set `self.isStuckToWall` true)
    (set `self.wall normal` (.x HitNormal))
    (set `CharacterMovementComponent.GravityScale` 0.0 _charactermovement :!label _label_5)
    (set `MovementComponent.Velocity` (0.0 0.0 0.0) _charactermovement)
    (`PaperFlipbookComponent.SetFlipbook` (`self.b_idle`) "/Game/flipbook/character/bunny/b_idle.b_idle")
    (set `self.hasJumped` false)
    (elif (`self.ActorHasTag` Other "ceiling")
      (set `self.Is Stuck on Ceiling` true)
      (set `self.ceiling normal` (.z HitNormal))
      (goto _label_5))))

(event `InputAction|Crouch`
  (params (Key :type "Key Structure"))
  (bind _returnvalue (`NavMovementComponent.IsFalling` (`self.CharacterMovement`)))
  ;[1 1 1] Crouch & Ground Pound
  (:`Pressed`
    (if _returnvalue
      (if (`self.canGroundPound`)
        (`self.GroundPound`))
      (else
        (`self.Crouch`))))
  (:`Released`
    (if (not _returnvalue)
      (`self.UnCrouch`))))

(fn `Death`
  (`KismetSystemLibrary.PrintString` "YOU DEAD."))

(fn `GroundPound`
  (set `self.isGroundPounding` true)
  (`PrimitiveComponent.SetPhysicsLinearVelocity` (`self.CapsuleComponent`) (0.0 0.0 0.0) false "None")
  (`self.LaunchCharacter` (0.0 0.0 -3000.0))
  (`KismetSystemLibrary.PrintString` "Ground Pound"))

(fn `UserConstructionScript`)
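; Player character pawn for a 2D flipbook platformer with walking, limited jumps and dashes, wall slide and wall jump, plus WIP health and enemy bounce.
; Player controller dispatchers drive the input events, which switch CharacterMovement into custom modes that UpdateCustomMovement executes.
; A toggled overlap volume detects "wall"-tagged actors to start sliding, and landing resets the jump and dash counters.
; Damage uses a timed DoOnce for invulnerability frames, and death only prints.
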(event `Setup Event`
  ;[1 1 1] Defaults
  (set `self.Current Life` (`self.Max Life`)))

(event `self.ReceiveBeginPlay`
  ;[1 1 1] Begin Play
  (`self.Setup Event`)
  (bind _aspob_player_controller (cast `/Game/Blueprints/characters/pob_playerController` (`GameplayStatics.GetPlayerController` 0)))
  (bind _output_get (set `self.pob_playerController` _aspob_player_controller))
  (`self.Bind Event` _output_get)
  (`self.Deactivate Wall Detect`))

(event `Bind Event`
  (params (`PoB Player Controller` :type "/Game/Blueprints/characters/pob_playerController Object Reference"))
  ;[1 1 1] Bind Events
  (add `/Game/Blueprints/characters/pob_playerController.jumpPressed` `PoB Player Controller` (delegate `jumpPressed_Event`))
  (add `/Game/Blueprints/characters/pob_playerController.jumpReleased` `PoB Player Controller` (delegate `jumpReleased_Event`))
  (add `/Game/Blueprints/characters/pob_playerController.DashPressed` `PoB Player Controller` (delegate `DashPressed_Event`))
  (add `/Game/Blueprints/characters/pob_playerController.walkingInput` `PoB Player Controller` (delegate `walkingInput_Event`))
  (add `self.Bunny Impact` (delegate `Bunny Impact_Event`))
  (`KismetSystemLibrary.Delay` 0.2)
  (`CharacterMovementComponent.SetMovementMode` (`self.CharacterMovement`) "MOVE_Walking" 0))

(event `jumpPressed_Event`
  ;[1 1 1] Jump Mode Change
  (if (< (`self.numberOfJumps`) (`self.JumpMaxCount`))
    (if (== (`self.Current Custom Movement Mode`) (`self.Wall Slide State`))
      (`self.Deactivate Wall Detect`)
      (`CharacterMovementComponent.SetMovementMode` (`self.CharacterMovement`) "MOVE_Custom" (`self.Wall Jump State`))
      (else
        (`self.Activate Wall Detect`)
        (`CharacterMovementComponent.SetMovementMode` (`self.CharacterMovement`) "MOVE_Custom" (`self.Jump State`))))))

(event `jumpReleased_Event`
  ;[1 1 1] Stop Jumping
  (`self.StopJumping`))

(event `DashPressed_Event`
  ;[1 1 1] Dash Mode Change
  (if (< (`self.Number of Dashes`) (`self.Dash Max Count`))
    (`self.Dash Mode Change`)))

(event `self.wallSlide_vol.OnComponentBeginOverlap`
  (params (OverlappedComponent :type "PrimitiveComponent Object Reference") (OtherActor :type "Actor Object Reference") (OtherComp :type "PrimitiveComponent Object Reference") (OtherBodyIndex :type Integer) (bFromSweep :type Boolean) (SweepResult :type "HitResult Structure (by ref)"))
  ;[1 1 1] Wall Detection
  (`|ExecutionSequence`
    (:`then_0`
      (if (`self.ActorHasTag` OtherActor "wall")
        (`CharacterMovementComponent.SetMovementMode` (`self.CharacterMovement`) "MOVE_Custom" (`self.Wall Slide State`))))
    (:`then_1`
      (if (== (`self.Current Custom Movement Mode`) (`self.Wall Slide State`))
        (if (`self.ActorHasTag` OtherActor "floor")
          (`self.Custom On Landed`))))))

(event `walkingInput_Event`
  (params (NewParam :type "Float (double-precision)"))
  ;[1 1 1] Walking Mode
  (if (`|EnumEquality` (`CharacterMovementComponent.MovementMode` (`self.CharacterMovement`)) "MOVE_Walking")
    (`self.Walking Movement` NewParam)
    (elif (not (== (`self.Current Custom Movement Mode`) (`self.Wall Slide State`)))
      (`self.Jumping Movement` NewParam))))

(event `self.OnLanded`
  (params (Hit :type "HitResult Structure (by ref)"))
  ;[1 1 1] On Landed
  (`self.Deactivate Wall Detect` :!label _label)
  (`self.Walking Mode`)
  (`CharacterMovementComponent.SetMovementMode` (`self.CharacterMovement`) "MOVE_Walking" 0))

(event `self.wallSlide_vol.OnComponentEndOverlap`
  (params (OverlappedComponent :type "PrimitiveComponent Object Reference") (OtherActor :type "Actor Object Reference") (OtherComp :type "PrimitiveComponent Object Reference") (OtherBodyIndex :type Integer))
  ;[1 1 1] Wall Detection
  (if (`self.ActorHasTag` OtherActor "wall")
    (`PaperFlipbookComponent.SetFlipbook` (`self.base`) "/Game/flipbook/character/bunny/b_fall.b_fall")
    (`CharacterMovementComponent.SetMovementMode` (`self.CharacterMovement`) "MOVE_Falling" 0)))

(event `Key|Gamepad_FaceButton_Top`
  (params (Key :type "Key Structure"))
  ;[1 1 1] Debug
)

(event `Custom On Landed`
  ;[1 1 1] On Landed
  (goto _label))

(event `self.ReceiveTick`
  (params (DeltaSeconds :type "Float (single-precision)"))
  ;[1 1 1] Debug
)

(event `self.K2_OnMovementModeChanged`
  (params (PrevMovementMode :type "EMovementMode Enum" :default "MOVE_None") (NewMovementMode :type "EMovementMode Enum" :default "MOVE_None") (PrevCustomMode :type Byte) (NewCustomMode :type Byte))
  ;[1 1 1] Custom Modes
  (set `self.Current Custom Movement Mode` NewCustomMode)
  (`self.Reset Wall Slide`))

(event `self.OnJumped`
  (bind _base (`self.base`))
  ;[1 1 1] On Jump
  (`PaperFlipbookComponent.SetFlipbook` _base "/Game/flipbook/character/bunny/b_jump.b_jump")
  (`KismetSystemLibrary.Delay` (`PaperFlipbook.GetTotalDuration` (`PaperFlipbookComponent.GetFlipbook` _base)))
  (`PaperFlipbookComponent.SetFlipbook` _base "/Game/flipbook/character/bunny/b_fall.b_fall"))

(event `self.OnWalkingOffLedge`
  (params (PreviousFloorImpactNormal :type "Vector Structure (by ref)") (PreviousFloorContactNormal :type "Vector Structure (by ref)") (PreviousLocation :type "Vector Structure (by ref)") (TimeDelta :type "Float (single-precision)"))
  ;[1 1 1] Activate Wall Detect when Falling off Ledge
  (`PaperFlipbookComponent.SetFlipbook` (`self.base`) "/Game/flipbook/character/bunny/b_fall.b_fall")
  (`KismetSystemLibrary.Delay` 0.2)
  (`self.Activate Wall Detect`))

(event `Reset Wall Slide`
  ;[1 1 1] Custom Modes
  (goto _label_3 :!via `Reset`))

(event `self.K2_UpdateCustomMovement`
  (params (DeltaTime :type "Float (single-precision)"))
  (bind _mesh (`self.Mesh`))
  ;[1 1 1] Custom Modes
  (if (== (`self.Current Custom Movement Mode`) (`self.Wall Slide State`))
    (`self.Right Left or Idle`
      (:`Idle`
        (`self.Wall Push Off`))
      (:`Right`
        (`SceneComponent.K2_SetRelativeRotation` _mesh (struct :`Yaw` 180.0) false false)
        (`PaperFlipbookComponent.SetFlipbook` (`self.base`) "/Game/flipbook/character/bunny/b_wallSlide.b_wallSlide" :!label _label_2)
        (if (== (`self.Current Custom Movement Mode`) (`self.Wall Slide State`))
          (`MovementComponent.StopMovementImmediately` (`self.CharacterMovement`))
          (`SceneComponent.K2_SetWorldTransform` (`self.CapsuleComponent`) (`KismetMathLibrary.MakeTransform` (`KismetMathLibrary.MakeVector` (.x (.location (`self.GetTransform`))) (.y (.location (`self.GetTransform`))) (- (.z (.location (`self.GetTransform`))) 5.0)) (.rotation (`self.GetTransform`)) (.scale (`self.GetTransform`))) false false)
          (`/Engine/EditorBlueprintResources/StandardMacros.DoOnce` false :!label _label_3
            (:`Completed`
              (set `self.numberOfJumps` 0)))
          (else
            (`MovementComponent.StopMovementImmediately` (`self.CharacterMovement`)))))
      (:`Left`
        (`SceneComponent.K2_SetRelativeRotation` :`self` _mesh)
        (goto _label_2)))
    (elif (== (`self.Current Custom Movement Mode`) (`self.Dash State`))
      (`self.Dash Mode`) ; Need to add a difference between Ground dash and Air Dash to tune them to be the same
      (`KismetSystemLibrary.Delay` 0.35 :!label _label_4)
      (`self.Activate Wall Detect`)
      (elif (== (`self.Current Custom Movement Mode`) (`self.Wall Jump State`))
        (`self.Wall Jump mode`)
        (goto _label_4)
        (elif (== (`self.Current Custom Movement Mode`) (`self.Jump State`))
          (`self.Jumping Mode`))))))

(event `Wall Push Off`
  (bind _returnvalue_x (`KismetMathLibrary.BreakVector` (`KismetMathLibrary.GetForwardVector` (`SceneComponent.K2_GetComponentRotation` (`self.Arrow1`)))))
  ;[1 1 1] Wall Push Off
  (`MovementComponent.StopMovementImmediately` (`self.CharacterMovement`))
  (`self.K2_SetActorTransform` (`KismetMathLibrary.MakeTransform` (`KismetMathLibrary.MakeVector` (`KismetMathLibrary.Lerp` (.x (.location (`self.GetTransform`))) (+ (.x (.location (`self.GetTransform`))) (* _returnvalue_x (`self.Drop Off Wall`))) (* (`GameplayStatics.GetWorldDeltaSeconds`) 20.0)) (.y (.location (`self.GetTransform`))) (.z (.location (`self.GetTransform`)))) (.rotation (`self.GetTransform`)) (.scale (`self.GetTransform`))))
  (`PaperFlipbookComponent.SetFlipbook` (`self.base`) "/Game/flipbook/character/bunny/b_fall.b_fall")
  (`CharacterMovementComponent.SetMovementMode` (`self.CharacterMovement`) "MOVE_Falling" 0))

(event `dashInput`
  (params (`Input Axis` :type "Float (double-precision)"))
  ;[1 1 1] Rotate Dash Towards Direction - WIP
)

(event `self.ReceiveAnyDamage`
  (params (Damage :type "Float (single-precision)") (DamageType :type "DamageType Object Reference") (InstigatedBy :type "Controller Object Reference") (DamageCauser :type "Actor Object Reference"))
  ;[1 1 1] Health - WIP
  (`/Engine/EditorBlueprintResources/StandardMacros.DoOnce` false :!label _label_5
    (:`Completed`
      (bind _output_get (set `self.Current Life` (- (`self.Current Life`) Damage)))
      (if (<= _output_get 0.0)
        (`self.Death`)
        (else
          (`KismetSystemLibrary.PrintString` (`KismetStringLibrary.Concat_StrStr` "Remaining Life = " (`KismetStringLibrary.Conv_DoubleToString` _output_get)))))
      (`KismetSystemLibrary.Delay` (`self.Invlun Frames`)) ; Bunny Invuln Frame
      (goto _label_5 :!via `Reset`))))

(event `Bunny Impact_Event` :!signature `self.Bunny Impact`
  (params (Velocity :type "Vector Structure"))
  ;[1 1 1] Bounce on Enemies - WIP
  (`self.Right Left or Idle`
    (:`Right`
      (`self.LaunchCharacter` (`KismetMathLibrary.MakeVector` (* (.x Velocity) -1.0) 0.0 (* (.z Velocity) -1.0))))
    (:`Left`
      (`self.LaunchCharacter` (`KismetMathLibrary.MakeVector` (`KismetMathLibrary.Abs` (.x Velocity)) 0.0 (`KismetMathLibrary.Abs` (.z Velocity)))))))

(fn `Activate Wall Detect`
  (`PrimitiveComponent.SetCollisionEnabled` (`self.wallSlide_vol`) "QueryOnly"))

(fn `CanJumpInternal`
  (returns (ReturnValue :type Boolean))
  (return true))

(fn `Dash Mode`
  (bind _pob_playercontroller (`self.pob_playerController`))
  (bind _dash_distance (`self.Dash Distance`))
  (`MovementComponent.StopMovementImmediately` (`self.CharacterMovement`))
  (`self.LaunchCharacter` (`KismetMathLibrary.MakeVector` (* (`/Game/Blueprints/characters/pob_playerController.H Direction` _pob_playercontroller) _dash_distance) 0.0 (* _dash_distance (`/Game/Blueprints/characters/pob_playerController.V Direction` _pob_playercontroller))) true true)
  (`PaperFlipbookComponent.SetFlipbook` (`self.base`) "/Game/flipbook/character/bunny/b_dash.b_dash"))

(fn `Deactivate Wall Detect`
  (`PrimitiveComponent.SetCollisionEnabled` (`self.wallSlide_vol`) "NoCollision"))

(fn `Death`
  (`KismetSystemLibrary.PrintString` "You haz ded!"))

(fn `Falling Mode`
  (`PaperFlipbookComponent.SetFlipbook` (`self.base`) "/Game/flipbook/character/bunny/b_fall.b_fall")
  (`KismetSystemLibrary.PrintString` "MOVE Falling"))

(fn `Jumping Mode`
  (if (< (`self.numberOfJumps`) (`self.JumpMaxCount`))
    (bind _result (`/Engine/EditorBlueprintResources/StandardMacros.IncrementInt` (`self.numberOfJumps`))
      (:`  `
        (set `self.numberOfJumps` _result)
        (`self.Jump`)))))

(fn `Jumping Movement`
  (params (InputPin :type "Float (double-precision)"))
  (bind _mesh (`self.Mesh`))
  (`self.Right Left or Idle`
    (:`Right`
      (`SceneComponent.K2_SetRelativeRotation` :`self` _mesh))
    (:`Left`
      (`SceneComponent.K2_SetRelativeRotation` _mesh (struct :`Yaw` 180.0) false false)))
  (`self.AddMovementInput` (1.0 0.0 0.0) InputPin))

(fn `UserConstructionScript`)

(fn `Walking Mode`
  (set `self.numberOfJumps` 0)
  (set `self.Number of Dashes` 0))

(fn `Walking Movement`
  (params (InputPin :type "Float (double-precision)"))
  (bind _mesh (`self.Mesh`))
  (`self.Right Left or Idle`
    (:`Idle`
      (`PaperFlipbookComponent.SetFlipbook` (`self.base`) "/Game/flipbook/character/bunny/b_idle.b_idle"))
    (:`Right`
      (`SceneComponent.K2_SetRelativeRotation` :`self` _mesh)
      (`self.AddMovementInput` (1.0 0.0 0.0) InputPin :!label _label)
      (`PaperFlipbookComponent.SetFlipbook` (`self.base`) "/Game/flipbook/character/bunny/b_walk.b_walk"))
    (:`Left`
      (`SceneComponent.K2_SetRelativeRotation` _mesh (struct :`Yaw` 180.0) false false)
      (goto _label))))

(fn `Wall Jump mode`
  (bind _returnvalue_x (`KismetMathLibrary.BreakVector` (`KismetMathLibrary.GetForwardVector` (`SceneComponent.K2_GetComponentRotation` (`self.Arrow1`)))))
  (`MovementComponent.StopMovementImmediately` (`self.CharacterMovement`))
  (`self.K2_SetActorTransform` (`KismetMathLibrary.MakeTransform` (`KismetMathLibrary.MakeVector` (`KismetMathLibrary.Lerp` (.x (.location (`self.GetTransform`))) (+ (.x (.location (`self.GetTransform`))) (* _returnvalue_x (`self.Drop Off Wall`))) (* (`GameplayStatics.GetWorldDeltaSeconds`) 20.0)) (.y (.location (`self.GetTransform`))) (.z (.location (`self.GetTransform`)))) (.rotation (`self.GetTransform`)) (.scale (`self.GetTransform`))))
  (`self.LaunchCharacter` (`KismetMathLibrary.MakeVector` (* _returnvalue_x -250.0) 0.0 (`self.Wall Jump Up Velocity`)) false true)
  (`PaperFlipbookComponent.SetFlipbook` (`self.base`) "/Game/flipbook/character/bunny/b_fall.b_fall"))
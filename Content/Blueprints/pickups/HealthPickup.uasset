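; Health pickup Blueprint that restores life to the player's bunny character, POB_CON_Bunny.
; Its PickupAction event casts the first player pawn to the bunny and adds HealthIncrease to CurrentLife, with no clamp in this graph, then prints the new total.
; Overlap and Tick events are disabled stubs, so nothing in this file triggers the action itself.
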(event `self.ReceiveBeginPlay`
  (`parent.ReceiveBeginPlay`))

(event `self.PickupAction`
  (bind _aspob_con_bunny (cast `/Game/Blueprints/characters/POB_CON_Bunny` (`GameplayStatics.GetPlayerPawn` 0)))
  (bind _output_get (set `/Game/Blueprints/characters/POB_CON_Bunny.CurrentLife` (+ (`/Game/Blueprints/characters/POB_CON_Bunny.CurrentLife` _aspob_con_bunny) (`self.HealthIncrease`)) _aspob_con_bunny))
  (`KismetSystemLibrary.PrintString` (`KismetStringLibrary.Concat_StrStr` "Remaining Life = " (`KismetStringLibrary.Conv_DoubleToString` _output_get))))

(fn `UserConstructionScript`
  (`parent.UserConstructionScript`))
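; Base pickup actor that is drawn toward the bunny player and collected on contact.
; On BeginPlay it scales its pickup range sphere by the player's PickupRangeMultiplier.
; Overlapping that sphere starts a per-tick lerp toward the player, which never stops because end overlap also sets IsInPickupRange true.
; An inner collection collision calls PickupAction, here only a debug print, then destroys the actor.
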(event `self.ReceiveTick`
  (params (DeltaSeconds :type "Float (single-precision)"))
  ;[1 1 1] Move Toward Player when in Range
  (if (`self.IsInPickupRange`)
    (`self.K2_SetActorLocation` (`KismetMathLibrary.VLerp` (`self.K2_GetActorLocation`) (`self.K2_GetActorLocation` (`GameplayStatics.GetPlayerPawn` 0)) (* DeltaSeconds 2.0)))))

(event `self.PickupRangeCollision.OnComponentBeginOverlap`
  (params (OverlappedComponent :type "PrimitiveComponent Object Reference") (OtherActor :type "Actor Object Reference") (OtherComp :type "PrimitiveComponent Object Reference") (OtherBodyIndex :type Integer) (bFromSweep :type Boolean) (SweepResult :type "HitResult Structure (by ref)"))
  ;[1 1 1] Collisions
  (if (== (`GameplayStatics.GetObjectClass` OtherActor) "/Game/Blueprints/characters/POB_CON_Bunny.POB_CON_Bunny_C")
    (set `self.IsInPickupRange` true)))

(event `self.PickupRangeCollision.OnComponentEndOverlap`
  (params (OverlappedComponent :type "PrimitiveComponent Object Reference") (OtherActor :type "Actor Object Reference") (OtherComp :type "PrimitiveComponent Object Reference") (OtherBodyIndex :type Integer))
  ;[1 1 1] Collisions
  (if (== (`GameplayStatics.GetObjectClass` OtherActor) "/Game/Blueprints/characters/POB_CON_Bunny.POB_CON_Bunny_C")
    (set `self.IsInPickupRange` true)))

(event `self.CollectionCollision.OnComponentBeginOverlap`
  (params (OverlappedComponent :type "PrimitiveComponent Object Reference") (OtherActor :type "Actor Object Reference") (OtherComp :type "PrimitiveComponent Object Reference") (OtherBodyIndex :type Integer) (bFromSweep :type Boolean) (SweepResult :type "HitResult Structure (by ref)"))
  ;[1 1 1] Collisions
  (if (== (`GameplayStatics.GetObjectClass` OtherActor) "/Game/Blueprints/characters/POB_CON_Bunny.POB_CON_Bunny_C")
    (`self.PickupAction`)
    (`self.K2_DestroyActor`)))

(event `self.ReceiveBeginPlay`
  (bind _pickuprangecollision (`self.PickupRangeCollision`))
  ;[1 1 1] Set Pickup Range Based on Player Multiplier
  (bind _aspob_con_bunny (cast `/Game/Blueprints/characters/POB_CON_Bunny` (`GameplayStatics.GetPlayerPawn` 0)))
  (`SphereComponent.SetSphereRadius` _pickuprangecollision (* (`SphereComponent.SphereRadius` _pickuprangecollision) (`/Game/Blueprints/characters/POB_CON_Bunny.PickupRangeMultiplier` _aspob_con_bunny)) true))

(fn `PickupAction`
  (`KismetSystemLibrary.PrintString` "Picked up"))

(fn `UserConstructionScript`)